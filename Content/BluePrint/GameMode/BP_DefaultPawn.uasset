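; Default pawn Blueprint that lets the player destroy the actor in the camera's line of sight with a left mouse click.
; A Visibility line trace runs forward from the player camera with a timed debug line.
; The hit actor is destroyed and an explosion particle spawns at the impact point.
; The Branch condition is constant true, so both actions run without checking for a hit.
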(event EventBeginPlay)

(event Collision|EventActorBeginOverlap
  (params (OtherActor :type Actor%20Object%20Reference)))

(event EventTick
  (params (DeltaSeconds :type Float%20%28single-precision%29)))

(event Input|MouseEvents|LeftMouseButton
  (params (Key :type Key%20Structure :default "None"))
  (bind _returnvalue (Game|GetPlayerCameraManager 0))
  (bind _returnvalue_2 (Camera|GetCameraLocation _returnvalue))
  (:Pressed
    (bind _outhit (Collision|LineTraceByChannel _returnvalue_2 (+ _returnvalue_2 (* (Math|Vector|GetForwardVector (Camera|GetCameraRotation _returnvalue)) 1e+04)) "TraceTypeQuery1" false 0 "ForDuration"))
    (if true
      (Actor|DestroyActor (.HitActor (Collision|BreakHitResult _outhit)))
      (Effects|SpawnEmitteratLocation "/Game/StarterContent/Particles/P_Explosion.P_Explosion" (.ImpactPoint (Collision|BreakHitResult _outhit))))))

(fn ConstructionScript)