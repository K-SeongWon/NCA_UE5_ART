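; BP_Actor is a configurable interactive prop with two swappable meshes and a Style value that selects its behavior.
; Construction assigns the meshes and, by Style, adds a colored spotlight, reveals lock text or enables physics.
; EV_Click dispatches by Style to toggle attachment to the first-person character's AttachPoint, toggle the light, or cycle the lock's displayed number.
; A collapsed timeline graph for moving or rotating Mesh1 is never executed.
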(event Custom|EV_Light
  ;[1 1 1] Light Event
  (bind _isa (Utilities|FlowControl|FlipFlop)
    (:A
      _)
    (:B
      _))
  (Rendering|SetVisibility (Variables|Default|GetSpotLight) _isa false))

(event Custom|EV_Attach
  ;[1 1 1] Attach Event
  (Utilities|FlowControl|FlipFlop
    (:A
      (bind _asbp_first_person_character (Utilities|Casting|CastToBP_FirstPersonCharacter (Game|Player|GetPlayerPawn 0)))
      (Transformation|AttachComponentToComponent (Variables|/Game/FirstPerson/Blueprints/BP_FirstPersonCharacter.BP_FirstPersonCharacter_C|GetAttach%20Point _asbp_first_person_character) "None" "KeepWorld" "KeepWorld" "KeepWorld" true))
    (:B
      (Transformation|DetachFromActor "KeepWorld" "KeepWorld" "KeepWorld"))))

(event Custom|EV_Click
  ;[1 1 1] Switch
  (switch int (Variables|Default|Getstyle)
    (:2
      (CallFunction|EVAttach))
    (:6
      (CallFunction|EVLight))
    (:7
      (|lock))
    (:8
      (CallFunction|EVAttach)
      (CallFunction|EVLight))))

(fn ConstructionScript
  (Components|StaticMesh|SetStaticMesh (Variables|Default|GetMesh1) (Variables|Default|GetNew%20Mesh_1))
  (Components|StaticMesh|SetStaticMesh (Variables|Default|GetMesh2) (Variables|Default|GetNew%20Mesh_2))
  (switch int (Variables|Default|Getstyle)
    (:6
      (|Light :!label _label))
    (:7
      (|Visible))
    (:8
      (goto _label))
    (:9
      (Physics|SetSimulatePhysics (Variables|Default|GetMesh1) true))))